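; Bomberman-style bomb actor that explodes on the grid map after a short delay, then destroys itself.
; BeginPlay resets its own cell through the GameInstance's map reference, then sweeps a cross sized by player 0's BombeRange.
; DestroyWall skips one cell status, spawns an actor on empty cells, and clears breakable ones before spawning.
; The mesh blocks all channels once an overlap ends; older inline blast logic remains disconnected.
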(event `self.ReceiveBeginPlay`
  (`KismetSystemLibrary.Delay` 1.0)
  (bind _asbpgame_instance (cast `/Game/Blueprints/BPGameInstance` (`GameplayStatics.GetGameInstance`)))
  (bind _mapreference (`/Game/Blueprints/BPGameInstance.MapReference` _asbpgame_instance))
  (bind _case (`/Game/Blueprints/Map/MapGestion.PosToCase` _mapreference (`SceneComponent.K2_GetComponentLocation` (`self.RootComponent`))))
  (bind _caseinfo (`/Game/Blueprints/Map/MapGestion.GetCaseInformation` _mapreference _case))
  (`/Game/Blueprints/Map/MapGestion.SetCaseContent` _mapreference _case (make `/Game/Case` "NewEnumerator21" (`.Content_19_FCECE7714AB0F625A2BEF485E0BFE404` (break `/Game/Case` _caseinfo))))
  (bind _asthird_person_character (cast `/Game/Blueprints/ThirdPerson/ThirdPersonCharacter` (`GameplayStatics.GetPlayerPawn` 0)))
  (bind _bomberange (`/Game/Blueprints/ThirdPerson/ThirdPersonCharacter.BombeRange` _asthird_person_character))
  (for _index (range (* _bomberange -1) (+ _bomberange 1))
    (bind _case_2 (`/Game/Blueprints/Map/MapGestion.PosToCase` _mapreference (`SceneComponent.K2_GetComponentLocation` (`self.RootComponent`))))
    (`|ExecutionSequence`
      (:`then_0`
        (`self.DestroyWall` _mapreference (`KismetMathLibrary.MakeVector2D` (`KismetMathLibrary.BreakVector2D` _case_2) (+ (`.Y` (`KismetMathLibrary.BreakVector2D` _case_2)) (`KismetMathLibrary.Conv_IntToDouble` _index)))))
      (:`then_1`
        (`self.DestroyWall` _mapreference (`KismetMathLibrary.MakeVector2D` (+ (`KismetMathLibrary.BreakVector2D` _case_2) (`KismetMathLibrary.Conv_IntToDouble` _index)) (`.Y` (`KismetMathLibrary.BreakVector2D` _case_2)))))))
  (`KismetSystemLibrary.Delay` 0.2)
  (`self.K2_DestroyActor`))

(event `self.StaticMesh.OnComponentEndOverlap`
  (params (OverlappedComponent :type "PrimitiveComponent Object Reference") (OtherActor :type "Actor Object Reference") (OtherComp :type "PrimitiveComponent Object Reference") (OtherBodyIndex :type Integer))
  ;[1 1 1] Block tout après la sortie du joueur
  (`PrimitiveComponent.SetCollisionResponseToAllChannels` (`self.StaticMesh`) "ECR_Block"))

(fn `DestroyWall`
  (params (MapGestion :type "/Game/Blueprints/Map/MapGestion Object Reference") (CasePos :type "Vector2D Structure"))
  (bind _caseinfo (`/Game/Blueprints/Map/MapGestion.GetCaseInformation` MapGestion (`KismetMathLibrary.MakeVector2D` CasePos_X CasePos_Y)))
  (if (`|EnumEquality` (break `/Game/Case` _caseinfo) "NewEnumerator18")
    _
    (elif (`|EnumEquality` (break `/Game/Case` _caseinfo) "NewEnumerator21")
      (bind _worldpos (`/Game/Blueprints/Map/MapGestion.CaseToWorldPos` MapGestion (`KismetMathLibrary.MakeVector2D` CasePos_X CasePos_Y) :!label _label))
      (`|SpawnActorFromClass` "/Game/Blueprints/Bombe/Explosion.Explosion_C" (`KismetMathLibrary.MakeTransform` _worldpos (struct)) "Undefined" "OverrideRootScale" null null)
      (elif (`|EnumEquality` (break `/Game/Case` _caseinfo) "NewEnumerator19")
        (`/Game/Blueprints/Map/MapGestion.SetCaseContent` MapGestion (`KismetMathLibrary.MakeVector2D` CasePos_X CasePos_Y) (make `/Game/Case` "NewEnumerator21" (`.Content_19_FCECE7714AB0F625A2BEF485E0BFE404` (break `/Game/Case` _caseinfo))))
        (bind _caseinfo_2 (`/Game/Blueprints/Map/MapGestion.GetCaseInformation` MapGestion (`KismetMathLibrary.MakeVector2D` CasePos_Y CasePos_X)))
        (`/Engine/EditorBlueprintResources/StandardMacros.IsValid` (`.Content_19_FCECE7714AB0F625A2BEF485E0BFE404` (break `/Game/Case` _caseinfo_2))
          (:`Is Valid`
            (`self.K2_DestroyActor` (`.Content_19_FCECE7714AB0F625A2BEF485E0BFE404` (break `/Game/Case` _caseinfo_2)))
            (goto _label))
          (:`Is Not Valid`
            (goto _label)))))))

(fn `UserConstructionScript`)