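; BP_Ennemies is an enemy Blueprint driven by a behavior tree.
; On BeginPlay it spawns its default AI controller and runs BT_Ennemies on it.
; Its Kill event passes the enemy to PlayerKill on the Game object held by BPGameInstance, then destroys the actor.
; If the game instance cast fails, the actor is not destroyed.
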(event `self.ReceiveBeginPlay`
  ;[1 1 1] initialise IA
  (`self.SpawnDefaultController`)
  (`AIController.RunBehaviorTree` (`AIBlueprintHelperLibrary.GetAIController` self) "/Game/Blueprints/IA/BT_Ennemies.BT_Ennemies"))

(event `Kill`
  ;[1 1 1] Kill event
  (bind _asbpgame_instance (cast `/Game/Blueprints/BPGameInstance` (`GameplayStatics.GetGameInstance`)))
  (`/Game/Blueprints/Game/GameGestion.PlayerKill` (`/Game/Blueprints/BPGameInstance.Game` _asbpgame_instance) self)
  (`self.K2_DestroyActor`))

(fn `UserConstructionScript`)