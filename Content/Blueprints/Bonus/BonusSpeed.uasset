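; Speed bonus pickup that raises a Base_Player's Speed by 0.5, up to a cap, when it overlaps.
; It rewrites the DataPlayer struct with the clamped Speed and a fixed 1 in the other field.
; It then spawns an enlarged TextRenderActor at the player with a French gain or limit message, testing the already updated Speed.
; The parent overlap handler runs last, only for players.
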(event `self.ReceiveActorBeginOverlap`
  (params (OtherActor :type "Actor Object Reference"))
  (bind _asbase_player (cast `/Game/Blueprints/Player/Base_Player` OtherActor))
  (bind (_dataplayer_numberlife _dataplayer_speed) (break `/Game/Blueprints/Player/DataPlayer` (`/Game/Blueprints/Player/Base_Player.DataPlayer` _asbase_player)))
  (bind _returnvalue (+ _dataplayer_speed 0.5))
  (bind _returnvalue_2 (`KismetMathLibrary.FMin` _returnvalue 4.0))
  (set `/Game/Blueprints/Player/Base_Player.DataPlayer` (make `/Game/Blueprints/Player/DataPlayer` 1 _returnvalue_2) _asbase_player)
  ;[1 1 1] Pop up texte
  (bind _returnvalue_3 (`|SpawnActorFromClass` "/Script/Engine.TextRenderActor" (`self.GetTransform` OtherActor) "Undefined" "OverrideRootScale" OtherActor null))
  (`self.K2_SetActorRotation` _returnvalue_3 (struct :`Yaw` 90.0) false)
  (bind _textrender (`TextRenderActor.TextRender` _returnvalue_3))
  (`TextRenderComponent.SetXScale` _textrender 5.0)
  (`TextRenderComponent.SetYScale` _textrender 5.0)
  (if (!= _returnvalue _returnvalue_2)
    (`TextRenderComponent.K2_SetText` _textrender (`KismetTextLibrary.Conv_StringToText` "Impossible d'augmenter sa vitesse"))
    (else
      (`TextRenderComponent.K2_SetText` _textrender (`KismetTextLibrary.Conv_StringToText` "Vitesse +1"))))
  (`parent.ReceiveActorBeginOverlap` OtherActor))

(event `self.ReceiveTick`
  (params (DeltaSeconds :type "Float (single-precision)"))
  (`parent.ReceiveTick` DeltaSeconds))

(fn `UserConstructionScript`
  (`parent.UserConstructionScript`))