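; BonusAddBomb is a pickup bonus that raises an overlapping player's bomb capacity by one.
; On actor overlap it casts the other actor to Base_Player and rebuilds its DataBombe struct with Count incremented, keeping Range, Timer and CanPush unchanged.
; It then calls the parent overlap event, so any further pickup behaviour is left to the parent class.
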(event `self.ReceiveActorBeginOverlap`
  (params (OtherActor :type "Actor Object Reference"))
  (bind _asbase_player (cast `/Game/Blueprints/Player/Base_Player` OtherActor))
  (bind (_databombe_range _databombe_timer _databombe_count _databombe_canpush) (break `/Game/Blueprints/Bombe/DataBombe` (`/Game/Blueprints/Player/Base_Player.DataBombe` _asbase_player)))
  (set `/Game/Blueprints/Player/Base_Player.DataBombe` (make `/Game/Blueprints/Bombe/DataBombe` _databombe_range _databombe_timer (+ _databombe_count 1) _databombe_canpush) _asbase_player)
  (`parent.ReceiveActorBeginOverlap` OtherActor))

(event `self.ReceiveTick`
  (params (DeltaSeconds :type "Float (single-precision)"))
  (`parent.ReceiveTick` DeltaSeconds))

(fn `UserConstructionScript`
  (`parent.UserConstructionScript`))