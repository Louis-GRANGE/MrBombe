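; Base player for a grid-based bomb game, handling bomb placement, lives and death.
; PutBomb routes through the server to a multicast that spawns a bomb snapped to the map cell, if the cell's status allows and the DataBombe count limit isn't reached.
; AddBombe frees a bomb slot.
; Kill removes a life, then grants brief invulnerability counted down on Tick, or reports death to the game when none remain.
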(event `MultiCastSpawnBombe`
  ;[0.4427 0 0.02768] SpawnBombe
  (bind _asbpgame_instance (cast `/Game/Blueprints/BPGameInstance` (`GameplayStatics.GetGameInstance`)))
  (bind _mapreference (`/Game/Blueprints/BPGameInstance.MapReference` _asbpgame_instance))
  (bind _case (`/Game/Blueprints/Map/MapGestion.PosToCase` _mapreference (`SceneComponent.K2_GetComponentLocation` (`self.DropBombe`))))
  (bind _caseinfo (`/Game/Blueprints/Map/MapGestion.GetCaseInformation` _mapreference _case))
  (if (`|EnumEquality` (break `/Game/Case` _caseinfo) "NewEnumerator21")
    (bind _canplace (`self.CanPlaceBomb`))
    (if _canplace
      (bind _worldpos (`/Game/Blueprints/Map/MapGestion.CaseToWorldPos` _mapreference _case))
      (`|SpawnActorFromClass` "/Game/Blueprints/Bombe/Bombe.Bombe_C" (`KismetMathLibrary.MakeTransform` _worldpos) "Undefined" "OverrideRootScale" null (`self.DataBombe`) self null)
      (`/Engine/EditorBlueprintResources/StandardMacros.IncrementInt` (`self.DroppedBombe`)))))

(event `RunServerSpawnBombe`
  ;[1 1 1] Spawn Bomb for network
  (`self.MultiCastSpawnBombe` :!label _label))

(event `PutBomb`
  ;[1 1 1] Spawn Bomb for network
  (`/Engine/EditorBlueprintResources/ActorMacros.Switch Has Authority`
    (:`Authority`
      (goto _label))
    (:`Remote`
      (`self.RunServerSpawnBombe`))))

(event `AddBombe`
  ;[1 1 1] Decrement droppped bombe
  (`/Engine/EditorBlueprintResources/StandardMacros.DecrementInt` (`self.DroppedBombe`)))

(event `self.ReceiveTick`
  (params (DeltaSeconds :type "Float (single-precision)"))
  ;[1 1 1] Enléve l'invulnérabilité si le joueur la possédent
  (bind _isinvu (`self.IsInvunarible`))
  (if _isinvu
    (set `self.TimerInvenurability` (- (`self.TimerInvenurability`) DeltaSeconds))))

(fn `CanPlaceBomb`
  (returns (canPlace :type Boolean))
  (bind (_databombe_range _databombe_timer _databombe_count) (break `/Game/Blueprints/Bombe/DataBombe` (`self.DataBombe`)))
  (return (< (`self.DroppedBombe`) _databombe_count)))

(fn `IsInvunarible`
  (returns (IsInvu :type Boolean))
  ;[1 1 1] Si le temps d'invunérabilité est supérieur à 0 il l'est donc
  (return (> (`self.TimerInvenurability`) 0.0)))

(fn `Kill`
  (returns (IsKill :type Boolean))
  (bind _dataplayer_numberlife (break `/Game/Blueprints/Player/DataPlayer` (`self.DataPlayer`)))
  ;[1 1 1] Event qui permet de tuer le joueur et ce supprime de la partie
  (bind _isinvu (`self.IsInvunarible`))
  (if _isinvu
    (return false)
    (else
      (bind _result (`/Engine/EditorBlueprintResources/StandardMacros.DecrementInt` _dataplayer_numberlife)
        (:`  `
          (if (< _result 1)
            (bind _asbpgame_instance (cast `/Game/Blueprints/BPGameInstance` (`GameplayStatics.GetGameInstance`)))
            (`/Game/Blueprints/Game/GameGestion.PlayerKill` (`/Game/Blueprints/BPGameInstance.Game` _asbpgame_instance) self)
            (return true)
            (else
              (set `self.TimerInvenurability` 1.0)
              (return false))))))))

(fn `UserConstructionScript`)