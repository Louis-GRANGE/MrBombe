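; Map manager that builds a Bomberman-style grid arena at BeginPlay and registers itself on BPGameInstance.
; It derives cell size from the map's scale, marks borders, spawns fixed pillars, and randomly spawns destructible walls outside the four corner spawn areas.
; A flattened CaseContent array stores each cell's status and actor.
; Helpers convert between world positions and cells, read or write cell content, and destroy walls.
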(event `self.ReceiveBeginPlay`
  (bind (_returnvalue_x _returnvalue_y) (`KismetMathLibrary.BreakVector` (`self.GetActorScale3D` (`self.Map`))))
  ;[1 1 1] Calcul les valeurs de la taille de la map et des cases
  (`self.SetMapLenght` (`KismetMathLibrary.MakeVector2D` _returnvalue_x _returnvalue_y))
  (`self.SetCaseSize`)
  ;[1 1 1] Initialise le contenu des cases
  (`self.InitialiseCaseContent`)
  ;[1 1 1] Set Map Reference on the Game Instance
  (bind _asbpgame_instance (cast `/Game/Blueprints/BPGameInstance` (`GameplayStatics.GetGameInstance`)))
  (set `/Game/Blueprints/BPGameInstance.MapReference` self _asbpgame_instance)
  (`WidgetBlueprintLibrary.SetInputMode_GameOnly` (`GameplayStatics.GetPlayerController` 0)))

(fn `AxePosToCase`
  (params (Position :type "Float (double-precision)") (Size :type "Float (double-precision)"))
  (returns (Case :type Integer))
  ;[1 1 1] Convertie la position en index de case en fonction de ça position et de la taille dans seulement un axe
  (return (`KismetMathLibrary.FTrunc` (/ Position Size))))

(fn `CaseToWorldPos`
  (params (Pos :type "Vector2D Structure"))
  (returns (WorldPos :type "Vector Structure"))
  (bind (_maplenght_x _maplenght_y) (`KismetMathLibrary.BreakVector2D` (`self.MapLenght`)))
  (bind (_casesize_x _casesize_y) (`KismetMathLibrary.BreakVector2D` (`self.CaseSize`)))
  (bind (_casecount_x _casecount_y) (`KismetMathLibrary.BreakVector2D` (`self.CaseCount`)))
  ;[1 1 1] Regarde que les index soit bien compris dans la taille du tableau
  (if (or (< Pos_X 0.0) (< Pos_Y 0.0) (> Pos_X _casecount_x) (> Pos_Y _casecount_y))
    (return (0.0 0.0 0.0))
    (else
      (return (`KismetMathLibrary.MakeVector` (- (- (* (+ Pos_X 1.0) _casesize_x) (/ _maplenght_x 2.0)) (/ _casesize_x 2.0)) (- (- (* (+ Pos_Y 1.0) _casesize_y) (/ _maplenght_y 2.0)) (/ _casesize_y 2.0)))))))

(fn `Destroy All Destructible Walls`
  (bind (_casecount_x _casecount_y) (`KismetMathLibrary.BreakVector2D` (`self.CaseCount`)))
  (for _index (range (+ (`KismetMathLibrary.FTrunc` _casecount_x) 1))
    (for _index_2 (range (+ (`KismetMathLibrary.FTrunc` _casecount_y) 1))
      (bind _caseinfo (`self.GetCaseInformation` (`KismetMathLibrary.MakeVector2D` (`KismetMathLibrary.Conv_IntToDouble` _index) (`KismetMathLibrary.Conv_IntToDouble` _index_2))))
      (if (`|EnumEquality` (break `/Game/Case` _caseinfo) "NewEnumerator19")
        (`self.K2_DestroyActor` (`.Content_19_FCECE7714AB0F625A2BEF485E0BFE404` (break `/Game/Case` _caseinfo)))))))

(fn `DestroyOnThisCase`
  (params (Case :type "Vector2D Structure"))
  (bind _caseinfo (`self.GetCaseInformation` (`KismetMathLibrary.MakeVector2D` Case_X Case_Y)))
  (`/Engine/EditorBlueprintResources/StandardMacros.IsValid` (`.Content_19_FCECE7714AB0F625A2BEF485E0BFE404` (break `/Game/Case` _caseinfo))
    (:`Is Valid`
      (`self.K2_DestroyActor` (`.Content_19_FCECE7714AB0F625A2BEF485E0BFE404` (break `/Game/Case` _caseinfo)))
      (`self.SetCaseContent` (`KismetMathLibrary.MakeVector2D` Case_X Case_Y) (make `/Game/Case` "NewEnumerator21"))
      (return))))

(fn `GetCaseInformation`
  (params (Case :type "Vector2D Structure"))
  (returns (CaseInfo :type "/Game/Case Structure"))
  (bind (_casecount_x _casecount_y) (`KismetMathLibrary.BreakVector2D` (`self.CaseCount`)))
  ;[1 1 1] Vérification que les index soit dans la plague des éléments
  (if (or (<= Case_X 0.0) (>= Case_X _casecount_x) (<= Case_Y 0.0) (>= Case_Y _casecount_y))
    (return)
    (else
      (return (`|GetArrayItem` (`self.CaseContent`) (`KismetMathLibrary.FTrunc` (+ Case_Y (* (`KismetMathLibrary.FTrunc` _casecount_x) Case_X))))))))

(fn `GetCasePlayer`
  (params (Player :type "Pawn Object Reference"))
  (returns (Case :type "Vector2D Structure"))
  ;[1 1 1] Permet de donner la case ou ce situe le joueur
  (bind _case (`self.PosToCase` (`self.K2_GetActorLocation` Player)))
  (return _case))

(fn `InitialiseCaseContent`
  (locals (NewLocalVar_1 :type Byte :default 0))
  (bind (_casecount_x _casecount_y) (`KismetMathLibrary.BreakVector2D` (`self.CaseCount`)))
  ;[1 1 1] Initialisation des boucle permettent d'instancier la map
  (for _index (range 1 (+ (`KismetMathLibrary.FTrunc` _casecount_x) 1))
    (for _index_2 (range 1 (+ (`KismetMathLibrary.FTrunc` _casecount_y) 1))
      ;[1 1 1] Verification de si le mur est un rebord ou non
      (bind _verif (`self.IsWallBorder` _index _index_2))
      (if _verif
        ;[1 1 1] Ajout d'un mur non destructible dans le tableau de contenu des cases
        (`KismetArrayLibrary.Array_Add` (`self.CaseContent`) (make `/Game/Case` "NewEnumerator18"))
        (else
          ;[1 1 1] Regarde si la case peut-être un mur destructible ou non
          (bind _verif_2 (`self.IsDestructibleWall` _index _index_2))
          (if _verif_2
            (bind _returnvalue (`KismetMathLibrary.Conv_IntToDouble` _index))
            (bind _returnvalue_2 (`KismetMathLibrary.Conv_IntToDouble` _index_2))
            ;[1 1 1] Vérifie que ce ne soit pas une case dans une zone d'apparition
            (bind _verif_3 (`self.IsSpawnArea` _returnvalue _returnvalue_2))
            (if _verif_3
              ;[1 1 1] Créer une case Vide
              (`KismetArrayLibrary.Array_Add` (`self.CaseContent`) (make `/Game/Case` "NewEnumerator21") :!label _label)
              (else
                ;[1 1 1] Prend une valeur aléatoire et regarde si elle est inférieur au seuil donnée
                (if (< (`KismetMathLibrary.RandomFloatInRange` 0.0 100.0) (`self.PercentageWallSpawn`))
                  ;[1 1 1] Créer un mur desctructible
                  (`self.SpawnDestructWall` _returnvalue _returnvalue_2)
                  (else
                    (goto _label)))))
            (else
              ;[1 1 1] Créer un mur indesctructible
              (`self.SpawnInDestructWall` _returnvalue _returnvalue_2))))))))

(fn `IsDestructibleWall`
  (params (X :type Integer) (Y :type Integer))
  (returns (Verif :type Boolean))
  (bind (_casecount_x _casecount_y) (`KismetMathLibrary.BreakVector2D` (`self.CaseCount`)))
  ;[1 1 1] Si la case à un des index est un modulo de 2, et qu'ils sont contraire à 0 ou la valeur max des cases, c'est qu'il peut créer un mur desctructible
  (return (and (or (== (mod X 2) 0) (== (mod Y 2) 0)) (> X 1) (< X (`KismetMathLibrary.FTrunc` _casecount_x)) (> Y 1) (< Y (`KismetMathLibrary.FTrunc` _casecount_y)))))

(fn `IsSpawnArea`
  (params (X :type "Float (double-precision)") (Y :type "Float (double-precision)"))
  (returns (verif :type Boolean))
  (locals (NewLocalVar_2 :type "Vector2D Structure") (NewLocalVar_3 :type "Vector2D Structure"))
  (bind _returnvalue (<= X 3.0))
  (bind _returnvalue_2 (<= Y 3.0))
  (bind (_casecount_x _casecount_y) (`KismetMathLibrary.BreakVector2D` (`self.CaseCount`)))
  (bind _returnvalue_3 (>= X (- _casecount_x 2.0)))
  (bind _returnvalue_4 (>= Y (- _casecount_y 2.0)))
  ;[1 1 1] Vérifie si les index sont des valeurs qui sont situé dans la zone d'apparition d'un joueur
  (return (or (and _returnvalue _returnvalue_2) (and _returnvalue _returnvalue_4) (and _returnvalue_3 _returnvalue_2) (and _returnvalue_3 _returnvalue_4))))

(fn `IsWallBorder`
  (params (X :type Integer) (Y :type Integer))
  (returns (Verif :type Boolean))
  (bind (_casecount_x _casecount_y) (`KismetMathLibrary.BreakVector2D` (`self.CaseCount`)))
  ;[1 1 1] Regarde si la position des valeurs est soit égal à 0 soit au maximum du nombre de Case
  (return (or (== X 1) (== X (`KismetMathLibrary.FTrunc` _casecount_x)) (== Y 1) (== Y (`KismetMathLibrary.FTrunc` _casecount_y)))))

(fn `PosToCase`
  (params (Pos :type "Vector Structure"))
  (returns (Case :type "Vector2D Structure"))
  (locals (NewLocalVar_0 :type "Vector Structure" :default (0.0 0.0 0.0)))
  (bind (_casesize_x _casesize_y) (`KismetMathLibrary.BreakVector2D` (`self.CaseSize`)))
  (bind (_maplenght_x _maplenght_y) (`KismetMathLibrary.BreakVector2D` (`self.MapLenght`)))
  (bind (_returnvalue_x _returnvalue_y) (`KismetMathLibrary.BreakVector` (+ Pos (`KismetMathLibrary.Conv_Vector2DToVector` (/ (`self.MapLenght`) 2.0)))))
  ;[1 1 1] Ajout de la moitier de la taille de la map pour que les valeurs soit absolument positive
  ;[1 1 1] Vérifie que les valeurs ne soit pas au dessus de la taille de la map
  (if (or (> _returnvalue_x _maplenght_x) (> _maplenght_y _returnvalue_y))
    ;[1 1 1] Convertir l'axe X et Y dans l'index du tableau
    (bind _case (`self.AxePosToCase` _returnvalue_x _casesize_x))
    (bind _case_2 (`self.AxePosToCase` _returnvalue_y _casesize_y))
    (return (`KismetMathLibrary.MakeVector2D` (`KismetMathLibrary.Conv_IntToDouble` _case) (`KismetMathLibrary.Conv_IntToDouble` _case_2)))
    (else
      ;[1 1 1] Valeur par défaut -1 -1
      (return (-1.0 -1.0)))))

(fn `SetCaseContent`
  (params (Case :type "Vector2D Structure") (`New Case Content` :type "/Game/Case Structure"))
  (bind (_casecount_x _casecount_y) (`KismetMathLibrary.BreakVector2D` (`self.CaseCount`)))
  (if (or (<= Case_X 0.0) (>= Case_X _casecount_x) (<= Case_Y 0.0) (>= Case_Y _casecount_y))
    (return)
    (else
      (`KismetArrayLibrary.Array_Set` (`self.CaseContent`) (`KismetMathLibrary.FTrunc` (+ Case_Y (* Case_X _casecount_x))) `New Case Content`)
      (return))))

(fn `SetCaseSize`
  ;[1 1 1] Permet de calculer la taille d'une case
  (set `self.CaseSize` (/ (`self.MapLenght`) (`self.CaseCount`))))

(fn `SetMapLenght`
  (params (Scale :type "Vector2D Structure"))
  ;[1 1 1] Calcul de la taille de la map
  (set `self.MapLenght` (* Scale 100.0)))

(fn `SpawnDestructWall`
  (params (X :type "Float (double-precision)") (Y :type "Float (double-precision)"))
  (bind (_casesize_x _casesize_y) (`KismetMathLibrary.BreakVector2D` (`self.CaseSize`)))
  (bind (_maplenght_x _maplenght_y) (`KismetMathLibrary.BreakVector2D` (`self.MapLenght`)))
  ;[1 1 1] Faire apparaitre le mur à la position calculé
  (bind _returnvalue (`|SpawnActorFromClass` "/Game/Blueprints/Map/Wall_Destructable.Wall_Destructable_C" (`KismetMathLibrary.MakeTransform` (`KismetMathLibrary.MakeVector` (- (- (* X _casesize_x) (/ _maplenght_x 2.0)) (/ _casesize_x 2.0)) (- (- (* Y _casesize_y) (/ _maplenght_y 2.0)) (/ _casesize_y 2.0)) 0.0)) "Undefined" "OverrideRootScale" null null))
  ;[1 1 1] Rajoute le mur dans la liste de case
  (`KismetArrayLibrary.Array_Add` (`self.CaseContent`) (make `/Game/Case` "NewEnumerator19" _returnvalue)))

(fn `SpawnInDestructWall`
  (params (X :type "Float (double-precision)") (Y :type "Float (double-precision)"))
  (bind (_casesize_x _casesize_y) (`KismetMathLibrary.BreakVector2D` (`self.CaseSize`)))
  (bind (_maplenght_x _maplenght_y) (`KismetMathLibrary.BreakVector2D` (`self.MapLenght`)))
  ;[1 1 1] Faire apparaitre le mur à la position calculé
  (bind _returnvalue (`|SpawnActorFromClass` "/Game/Blueprints/Map/Wall_Indesctructable.Wall_Indesctructable_C" (`KismetMathLibrary.MakeTransform` (`KismetMathLibrary.MakeVector` (- (- (* X _casesize_x) (/ _maplenght_x 2.0)) (/ _casesize_x 2.0)) (- (- (* Y _casesize_y) (/ _maplenght_y 2.0)) (/ _casesize_y 2.0)) 160.0)) "Undefined" "OverrideRootScale" null null))
  ;[1 1 1] Rajoute le mur dans la liste de case
  (`KismetArrayLibrary.Array_Add` (`self.CaseContent`) (make `/Game/Case` "NewEnumerator18" _returnvalue)))

(fn `UserConstructionScript`)